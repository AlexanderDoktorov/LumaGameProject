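; Actor component for foliage bending that publishes player pawn position to materials.
; Each tick it smooths the owner's normalized speed and eases a trail point toward a spot behind the owner, following more slowly at low speed.
; It writes only player pawn 0's location to the Location1 collection parameter; the smoothed speed and trail point are not sent to materials here.
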(event EventTick
  (params (DeltaSeconds :type Float%20%28single-precision%29))
  (bind _returnvalue (Components|GetOwner))
  (bind _character_max_speed (Variables|Default|GetCharacter%20Max%20Speed))
  (Variables|Default|SetActorSpeed (Math|Interpolation|FInterpTo (Variables|Default|GetActorSpeed) (/ (Math|Float|Clamp(Float) (Math|Vector|VectorLength (Transformation|GetVelocity (Components|GetOwner))) 0.0 _character_max_speed) _character_max_speed) (Utilities|Time|GetWorldDeltaSeconds) 1.5))
  (Variables|Default|SetTrailPos (Math|Interpolation|VInterpTo (Variables|Default|GetTrailPos) (+ (Transformation|GetActorLocation _returnvalue) (* (Math|Vector|NegateVector (Transformation|GetActorForwardVector _returnvalue)) (Variables|Default|GetPath%20Length))) (Utilities|Time|GetWorldDeltaSeconds) (Math|Float|SelectFloat 1.0 5.0 (< (Math|Vector|VectorLength (Transformation|GetVelocity _returnvalue)) (/ (Variables|Default|GetCharacter%20Max%20Speed) 5.0)))))
  (Rendering|Material|SetVectorParameterValue "/Game/Game/Materials/Demo/MaterialParameterCollection.MaterialParameterCollection" "Location1" (Math|Conversions|ToLinearColor(Vector) (Transformation|GetActorLocation (Game|Player|GetPlayerPawn 0))) :!class /Script/Engine.KismetMaterialLibrary))