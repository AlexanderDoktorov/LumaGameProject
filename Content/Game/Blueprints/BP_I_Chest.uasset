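; Interactable treasure chest that shows an on-screen prompt to a nearby player and can spawn loot when opening starts.
; Box overlap creates the prompt if the character allows it and the chest's AnimInstance reports unopened, retrying by timer when disallowed.
; A looping timer pins the widget to the chest's projected screen position.
; Interface functions supply interaction rules; starting interaction removes the prompt and optionally scatters loot classes once.
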(event OnComponentBeginOverlap(Box)
  (params (OverlappedComponent :type Primitive%20Component%20Object%20Reference) (OtherActor :type Actor%20Object%20Reference) (OtherComp :type Primitive%20Component%20Object%20Reference) (OtherBodyIndex :type Integer) (bFromSweep :type Boolean) (SweepResult :type Hit%20Result%20Structure%20%28by%20ref%29))
  ;[1 1 1] Generate Widget
  (InfoWidget|Widget-Generate OtherActor))

(event OnComponentEndOverlap(Box)
  (params (OverlappedComponent :type Primitive%20Component%20Object%20Reference) (OtherActor :type Actor%20Object%20Reference) (OtherComp :type Primitive%20Component%20Object%20Reference) (OtherBodyIndex :type Integer))
  ;[1 1 1] Generate Widget
  (InfoWidget|Widget-Destroy))

(event Custom|CheckWhdgetWhenInTrigger
  (bind _box (Variables|Default|GetBox))
  (bind _overlappingactors (Collision|GetOverlappingActors _box "/Script/Engine.Character" :!class /Script/Engine.PrimitiveComponent))
  ;[1 1 1] Generate Widget
  (if (> (Utilities|Array|Length _overlappingactors) 0)
    (InfoWidget|Widget-Generate (Utilities|Array|Get(acopy) _overlappingactors))))

(event Custom|Widget%20Update%20Event
  ;[1 1 1] Generate Widget
  (InfoWidget|Widget-Update))

(event EventDestroyed
  ;[1 1 1] Generate Widget
  (InfoWidget|Widget-Destroy))

(event EventBPISetInteractionState
  (params (StartedInteract :type Boolean) (Param :type Boolean))
  (bind _output_get (Variables|Default|SetStartedOpenMontage StartedInteract))
  (if (and _output_get (Variables|Config|GetLootsItemsSpawnWhenOpen))
    (TryOpen|SpawnLootItems))
  (InfoWidget|Widget-Destroy))

(fn ConstructionScript)

(fn Widget-Generate
  (params (Actor :type Actor%20Object%20Reference))
  (bind _ascharacter (Utilities|Casting|CastToCharacter Actor))
  (LocalVariables|SetCharacter _ascharacter)
  (if (Pawn|IsPlayerControlled _ascharacter)
    (bind _returnvalue (Class|ALSPlayerCharacterBPI|PBPICheckItemCanSpawnWidget(Message) (LocalVariables|GetCharacter) self (Transformation|GetActorLocation)))
    (if _returnvalue
      (if (and (InfoWidget|ChestIsCurrentNotOpened) (not (Variables|InfoWidget|GetGeneratedInfoWidget)))
        ;[1 1 1] Spawn Widget
        (bind _returnvalue_2 (UserInterface|CreateWidget "/Game/AdvancedLocomotionV4/Blueprints/UI/Item_Information_UI.Item_Information_UI_C"))
        (bind _output_get (Variables|InfoWidget|SetInfoWidgetObject _returnvalue_2))
        (UserInterface|Viewport|AddtoViewport _output_get -1)
        (Variables|InfoWidget|SetGeneratedInfoWidget true)
        (UserInterface|Animation|PlayAnimation (Variables|InfoWidget|GetInfoWidgetObject) (Variables|/Game/AdvancedLocomotionV4/Blueprints/UI/Item_Information_UI.Item_Information_UI_C|GetFade_In (Variables|InfoWidget|GetInfoWidgetObject)) 0.0 1 "Forward" 1.4 false)
        (Utilities|FlowControl|Sequence
          (:then_0
            ;[1 1 1] Updare String
            (Rendering|Components|TextRender|SetText (Variables|/Game/AdvancedLocomotionV4/Blueprints/UI/Item_Information_UI.Item_Information_UI_C|GetT_Title (Variables|InfoWidget|GetInfoWidgetObject)) "")
            (Rendering|Components|TextRender|SetText (Variables|/Game/AdvancedLocomotionV4/Blueprints/UI/Item_Information_UI.Item_Information_UI_C|GetT_Comment (Variables|InfoWidget|GetInfoWidgetObject)) "")
            (Widget|SetRenderOpacity (Variables|/Game/AdvancedLocomotionV4/Blueprints/UI/Item_Information_UI.Item_Information_UI_C|GetBG_Blur (Variables|InfoWidget|GetInfoWidgetObject)) 0.0))
          (:then_1
            ;[1 1 1] Play Animation
            (UserInterface|Animation|PlayAnimation (Variables|InfoWidget|GetInfoWidgetObject) (Variables|/Game/AdvancedLocomotionV4/Blueprints/UI/Item_Information_UI.Item_Information_UI_C|GetButton_Loop (Variables|InfoWidget|GetInfoWidgetObject)) 0.0 15 "Forward" 1.4 false)
            (Utilities|Time|SetTimerbyFunctionName 0 "Widget Update Event" 0.01 true))
          (:then_2
            ;[1 0 0.3537] Activate Tick Per Frame
            (Class|ActorComponent|SetComponentTickInterval (Variables|Default|GetSK_TreasureChest) 0.0)))
        (else
          (return false)))
      (else
        (Utilities|Time|SetTimerbyFunctionName 0 "CheckWhdgetWhenInTrigger" 0.5)
        (return false)))
    (else
      (return false))))

(fn Widget-Update
  (if (and (Variables|InfoWidget|GetGeneratedInfoWidget) (Utilities|IsValid (Variables|InfoWidget|GetInfoWidgetObject)))
    (Utilities|Time|ClearTimerbyFunctionName 0 "CheckWhdgetWhenInTrigger")
    (Class|CanvasPanelSlot|SetPosition (Class|WidgetLayoutLibrary|SlotasCanvasSlot (Variables|/Game/AdvancedLocomotionV4/Blueprints/UI/Item_Information_UI.Item_Information_UI_C|GetMovablePanel (Variables|InfoWidget|GetInfoWidgetObject))) (.ScreenPosition (Class|WidgetLayoutLibrary|ProjectWorldLocationtoWidgetPosition (Widget|GetOwningPlayer (Variables|InfoWidget|GetInfoWidgetObject)) (+ (Transformation|GetWorldLocation (Variables|Default|GetWidgetOriring)) "0, 0, 0") false)))
    (else
      (Utilities|Time|ClearTimerbyFunctionName 0 "Widget Update Event"))))

(fn Widget-Destroy
  (Variables|InfoWidget|GetInfoWidgetObject
    (:then
      (Widget|SetVisibility (Variables|InfoWidget|GetInfoWidgetObject) "Hidden")
      (Widget|RemovefromParent (Variables|InfoWidget|GetInfoWidgetObject))
      (Variables|InfoWidget|SetGeneratedInfoWidget false)
      (Variables|InfoWidget|SetInfoWidgetObject 0)
      (Utilities|Time|ClearTimerbyFunctionName 0 "CheckWhdgetWhenInTrigger"))
    (:else)))

(fn ChestIsCurrentNotOpened
  (bind _returnvalue (Class|BPIItemswithAnimsInterface|BPIAnimGetChangeState(Message) (Components|SkeletalMesh|GetAnimInstance (Variables|Default|GetSK_TreasureChest))))
  (return (not _returnvalue)))

(fn SpawnLootItems
  (bind _spawningmaxoffset (Variables|Config|GetSpawningMaxOffset))
  (for _array_element (Variables|Config|GetLootsClass)
    (if (Utilities|IsValidClass _array_element)
      (Game|SpawnActorfromClass _array_element (Math|Transform|MakeTransform (+ (.OutPointOnBody (Collision|GetClosestPointonCollision (Variables|Default|GetSK_TreasureChest) (+ (- (Transformation|GetWorldLocation (Variables|Default|GetItemsSpawnOrigin)) "0,0,10.000000") (+ (* (Transformation|GetActorForwardVector) (* (Math|Random|RandomFloatinRange -1.0 1.0) (.y _spawningmaxoffset))) (* (Transformation|GetActorRightVector) (* (Math|Random|RandomFloatinRange 0.5 -1.0) (.x _spawningmaxoffset))))) "None")) "0.0,0.0,3.0") (Math|Rotator|CombineRotators (Transformation|GetActorRotation) (Math|Rotator|MakeRotator 0.0 0.0 (.yaw (Math|Random|RandomRotator false))))) "AlwaysSpawn" "SelectDefaultAtRuntime" 0 0)))
  (Utilities|Array|Clear (Variables|Config|GetLootsClass)))

(fn BPIActorStartedInteraction
  (return (Variables|Default|GetStartedOpenMontage)))

(fn BPIConfigHoldingOption
  (return false "NewEnumerator0"))

(fn BPIGetInteractionType
  (return "NewEnumerator1"))

(fn BPIGetInteractObjectConfig
  (return true true "(X=-75.000000,Y=75.000000)" "(X=-120.000000,Y=20.000000)" 1.8e+02 false false 0))

(fn BPIGetItemtoPickType
  (return "None"))

(fn BPIGetManualVelocity
  (return "0, 0, 0"))

(fn BPIGetObjectCollisionOverlap
  (params (ToIgnore :type Array%20of%20Actor%20Object%20References))
  (return false))

(fn BPIGetObjectTagContainer
  (return "(GameplayTags=((TagName=\"Interaction.OpenProp.Chest\")))"))

(fn BPIGetObjectTraceOrigin
  (return "0, 0, 0"))