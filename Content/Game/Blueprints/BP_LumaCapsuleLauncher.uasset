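; BP_LumaCapsuleLauncher is a launcher Blueprint that propels each bullet it spawns with a physics impulse.
; On the bullet spawn event, it finds the bullet's primitive component and, if valid, applies an impulse at the bullet's location.
; The impulse points along the launcher's right vector, with BulletLaunchStrengthK expressing strength in thousands.
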(event EventOnBulletSpawn
  (params (Bullet :type Actor%20Object%20Reference))
  (bind _returnvalue (Actor|GetComponentbyClass Bullet "/Script/Engine.PrimitiveComponent"))
  (Utilities|IsValid _returnvalue
    (:Is%20Valid
      (Physics|AddImpulseatLocation _returnvalue (* (* (Variables|Default|GetBullet%20Launch%20Strength%20%28k%29) (Transformation|GetActorRightVector)) (Math|Float|MakeLiteralFloat 1e+03)) (Transformation|GetActorLocation Bullet) "None"))))

(fn ConstructionScript
  (|CallParentFunction))