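; GA_ProximityMineKnockback is a gameplay ability that knocks back a character hit by a proximity mine explosion.
; It activates from a gameplay event, casting the event target to Character and the optional object to ProximityMine, and cancels if either cast fails.
; ApplyKnockback starts ragdoll through an interface message, then adds a configurable-strength impulse to the pelvis, directed away from the mine, before the ability ends.
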(event Ability|EventActivateAbilityFromEvent
  (params (EventData :type Gameplay%20Event%20Data%20Structure%20%28by%20ref%29))
  (bind (_eventtag _instigator _target _optionalobject) (Utilities|Struct|BreakGameplayEventData EventData))
  (Development|PrintString (Utilities|String|Append (Utilities|GetObjectName _target) " has been affected by proximity mine explosion"))
  (bind _ascharacter (Utilities|Casting|CastToCharacter _target)
    (:then
      (bind _asproximity_mine (Utilities|Casting|CastToProximityMine _optionalobject)
        (:then
          (CallFunction|ApplyKnockback _ascharacter _asproximity_mine)
          (Ability|EndAbility))
        (:CastFailed
          (Ability|CancelAbility))))
    (:CastFailed
      (Ability|CancelAbility))))

(fn ApplyKnockback
  (params (Character%20Target :type Character%20Object%20Reference) (Proximity%20Mine :type Proximity%20Mine%20Object%20Reference))
  ;[0 1 0.1356] Enables ragdoll and applies impules to pelvis in the direction from the sphere. Force strength is configurable.
  (Utilities|FlowControl|Sequence
    (:then_0
      (Class|ALSPlayerCharacterBPI|PBPIRagdollStartEnd(Message) Character%20Target true))
    (:then_1
      (Physics|AddImpulse (Variables|/Script/Engine.Character|GetMesh Character%20Target) (* (Math|Vector|Normalize (- (Transformation|GetWorldLocation (Variables|/Script/Engine.Character|GetCapsuleComponent Character%20Target)) (Transformation|GetWorldLocation (Variables|/Script/Interaction_With_ALS.ProximityMine|GetMesh Proximity%20Mine)))) (Variables|Default|GetKnockback%20Strength)) "pelvis" false))))