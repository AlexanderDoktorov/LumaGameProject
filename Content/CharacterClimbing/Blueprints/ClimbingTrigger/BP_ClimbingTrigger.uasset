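; Trigger actor that marks a climb spot and registers itself with an overlapping Character's climbing component while active.
; It passes its climb tag when climbing is possible, optionally starts the climb on touch, and can deactivate after use.
; A timeline rotates the character to the climb direction and can move it to that point or line, while looping timers apply timed capsule offsets.
; The construction script lists climb names from DT_ClimbingList.
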(event OnComponentBeginOverlap(TriggerCollision)
  (params (OverlappedComponent :type Primitive%20Component%20Object%20Reference) (OtherActor :type Actor%20Object%20Reference) (OtherComp :type Primitive%20Component%20Object%20Reference) (OtherBodyIndex :type Integer) (bFromSweep :type Boolean) (SweepResult :type Hit%20Result%20Structure%20%28by%20ref%29))
  ;[1 1 1] Trigger
  (Utilities|CheckIsActive
    (:IsActive
      (bind _ascharacter (Utilities|Casting|CastToCharacter OtherActor))
      (bind _output_get (Variables|Components|SetCharacter _ascharacter))
      (bind _climbingcomp (Class|BIClimbing|GetClimbingComp(Message) _output_get))
      (Utilities|IsValid _climbingcomp
        (:Is%20Valid
          (Utilities|Array|AddUnique (Variables|/Game/CharacterClimbing/Blueprints/Climbing/BP_ClimbingComp.BP_ClimbingComp_C|GetCurrentClimbTriggers _climbingcomp) self)
          (if (Variables|/Game/CharacterClimbing/Blueprints/Climbing/BP_ClimbingComp.BP_ClimbingComp_C|GetCanClimbing _climbingcomp)
            (Variables|/Game/CharacterClimbing/Blueprints/Climbing/BP_ClimbingComp.BP_ClimbingComp_C|SetClimbTag _climbingcomp (Variables|Settings|GetClimbTag))
            (if (Variables|Settings|GetActivateByTouch)
              (Default|StartClimb _climbingcomp (Variables|Settings|GetForcedActivate)))))))))

(event OnComponentEndOverlap(TriggerCollision)
  (params (OverlappedComponent :type Primitive%20Component%20Object%20Reference) (OtherActor :type Actor%20Object%20Reference) (OtherComp :type Primitive%20Component%20Object%20Reference) (OtherBodyIndex :type Integer))
  ;[1 1 1] Trigger
  (bind _ascharacter (Utilities|Casting|CastToCharacter OtherActor))
  (Utilities|IsValid _ascharacter
    (:Is%20Valid
      (bind _climbingcomp (Class|BIClimbing|GetClimbingComp(Message) _ascharacter))
      (Utilities|IsValid _climbingcomp
        (:Is%20Valid
          (Utilities|Array|RemoveItem (Variables|/Game/CharacterClimbing/Blueprints/Climbing/BP_ClimbingComp.BP_ClimbingComp_C|GetCurrentClimbTriggers _climbingcomp) self))))))

(event Custom|OnClimbStart
  (Current|DeactivateAfterUseClimb)
  (Default|CallClimbActivate))

(event EventBeginPlay)

(event Collision|EventActorBeginOverlap
  (params (OtherActor :type Actor%20Object%20Reference)))

(event EventTick
  (params (DeltaSeconds :type Float%20%28single-precision%29)))

(fn ConstructionScript
  (bind _outrownames (DataTable|GetDataTableRowNames "/Game/CharacterClimbing/Blueprints/Climbing/DT_ClimbingList.DT_ClimbingList"))
  (Variables|Settings|SetClimbingList _outrownames))

(fn DeactivateAfterUseClimb
  (if (Variables|Settings|GetDeactivateAfterUse)
    (Variables|Settings|SetActive false)))

(fn CalcTargetLoc
  (bind _character (Variables|Components|GetCharacter))
  (bind _climbdirection (Variables|Default|GetClimbDirection))
  (bind _climbdirection_2 (Variables|Default|GetClimbDirection))
  (bind _character_2 (Variables|Components|GetCharacter))
  (bind _climbdirection_3 (Variables|Default|GetClimbDirection))
  (bind _returnvalue (Transformation|GetActorLocation _character_2))
  (bind _returnvalue_2 (Transformation|GetWorldLocation _climbdirection))
  (bind _returnvalue_3 (Transformation|GetActorLocation _character))
  (bind _returnvalue_4 (Transformation|GetWorldLocation _climbdirection_2))
  (bind _returnvalue_5 (Math|Vector|GetRightVector _climbdirection_3))
  (bind _returnvalue_6 (Math|Vector|FindClosestPointonLine _returnvalue _returnvalue_4 _returnvalue_5))
  (if (Variables|Settings|GetMoveToDirectionLine)
    (Variables|Current|SetTargetCharLoc (Math|Vector|MakeVector (.x _returnvalue_6) (.y _returnvalue_6) (select (Variables|Settings|GetUseZLoc) (.z _returnvalue_6) (.z _returnvalue_3))))
    (else
      (Variables|Current|SetTargetCharLoc (Math|Vector|MakeVector (.x _returnvalue_2) (.y _returnvalue_2) (select (Variables|Settings|GetUseZLoc) (.z _returnvalue_2) (.z _returnvalue_3)))))))

(event Custom|TransformCharacter
  (params (Delay :type Float%20%28double-precision%29) (RotateTime :type Float%20%28double-precision%29))
  (bind _character (Variables|Components|GetCharacter))
  (Utilities|FlowControl|RetriggerableDelay Delay)
  (Components|Timeline|SetPlayRate (Variables|Default|GetTM_RotateCharToClimbDirection) (/ 1.0 RotateTime))
  (Variables|Current|SetCurrentCharRot (Transformation|GetActorRotation _character))
  (if (Variables|Settings|GetCharacterMoveToPoint)
    (Variables|Current|SetCurrentCharLoc (Transformation|GetActorLocation _character))
    (Current|CalcTargetLoc)
    (bind _alpha (Timeline|TM_RotateCharToClimbDirection PlayFromStart)
      (:Update
        (Transformation|SetActorRotation (Variables|Components|GetCharacter) (Math|Rotator|MakeRotator 0.0 0.0 (.yaw (Math|Rotator|Lerp(Rotator) (Variables|Current|GetCurrentCharRot) (Transformation|GetWorldRotation (Variables|Default|GetClimbDirection)) _alpha true))))
        (if (Variables|Settings|GetCharacterMoveToPoint)
          (Transformation|SetActorLocation (Variables|Components|GetCharacter) (Math|Vector|Lerp(Vector) (Variables|Current|GetCurrentCharLoc) (Variables|Current|GetTargetCharLoc) _alpha) true false))))
    (else
      (Timeline|TM_RotateCharToClimbDirection PlayFromStart))))

(event Custom|MoveChar
  (params (Delay :type Float%20%28double-precision%29) (Time :type Float%20%28double-precision%29) (Direction :type Vector))
  (Utilities|FlowControl|RetriggerableDelay Delay)
  (bind _returnvalue (Utilities|Time|SetTimerbyEvent (delegate Custom|MoveCharUpdate) (/ (Utilities|Time|GetWorldDeltaSeconds) (Class|GameplayStatics|GetGlobalTimeDilation)) true))
  (Variables|Current|SetTimer_MoveChar _returnvalue)
  (bind _returnvalue_2 (Utilities|Time|SetTimerbyEvent (delegate Custom|ResetTimer) Time))
  (Variables|Current|SetTimer_ResetMoveChar _returnvalue_2))

(event Custom|MoveCharUpdate
  (Transformation|AddLocalOffset (Variables|/Script/Engine.Character|GetCapsuleComponent (Variables|Components|GetCharacter)) (stale Custom|MoveChar Direction) true false))

(event Custom|ResetTimer
  (Utilities|Time|ClearandInvalidateTimerbyHandle (Variables|Current|GetTimer_ResetMoveChar))
  (Utilities|Time|ClearandInvalidateTimerbyHandle (Variables|Current|GetTimer_MoveChar)))