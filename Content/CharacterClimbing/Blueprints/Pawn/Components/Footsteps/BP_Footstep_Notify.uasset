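; Animation notify that plays a footstep sound for the left or right foot of a character.
; It gets the footsteps component from the owning Character, line traces at the foot bone, and looks up the hit physical material's surface type in that component's CurrentFootsteps map.
; The matching sound spawns attached to the foot; a failed cast, missing component or missed trace plays the default CueFootStep at the foot's location instead.
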(fn ReceivedNotify
  (params (MeshComp :type Skeletal%20Mesh%20Component%20Object%20Reference) (Animation :type Anim%20Sequence%20Base%20Object%20Reference) (EventReference :type Anim%20Notify%20Event%20Reference%20Structure%20%28by%20ref%29))
  (bind _ascharacter (Utilities|Casting|CastToCharacter (Components|GetOwner MeshComp))
    (:then
      (LocalVariables|SetFootName (select (Variables|Settings|GetRightFoot?) (Variables|Settings|GetRightFootBoneName) (Variables|Settings|GetLeftFootBoneName)))
      (bind _footstepscomponent (Class|BIFootsteps|GetFootstepsComponent(Message) _ascharacter))
      (Utilities|IsValid _footstepscomponent
        (:Is%20Valid
          (bind (_outhit _returnvalue) (Collision|LineTraceByChannel (.Start (|FootTraceLoc MeshComp (LocalVariables|GetFootName))) (.End (|FootTraceLoc MeshComp (LocalVariables|GetFootName))) "TraceTypeQuery1" false 0 "None"))
          (if _returnvalue
            (Audio|SpawnSoundAttached (.Value (Utilities|Map|Find (Variables|/Game/CharacterClimbing/Blueprints/Pawn/Components/Footsteps/BP_Footstep_Comp.BP_Footstep_Comp_C|GetCurrentFootsteps _footstepscomponent) (Variables|/Script/PhysicsCore.PhysicalMaterial|GetSurfaceType (.PhysMat (Collision|BreakHitResult _outhit))))) MeshComp (LocalVariables|GetFootName) "0, 0, 0" "0, 0, 0" "KeepRelativeOffset" false 1.0 1.0 0.0 0 0)
            (else
              (Audio|PlaySoundatLocation (Variables|Settings|GetCueFootStep) (Transformation|GetSocketLocation MeshComp (LocalVariables|GetFootName)) "0, 0, 0" 1.0 1.0 0.0 0 0 0 0 :!label _label))))
        (:Is%20Not%20Valid
          (goto _label))))
    (:CastFailed
      (goto _label)))
  (return false))